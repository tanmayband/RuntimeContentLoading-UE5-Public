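; BP_PakLoader is an admin actor that loads and clears external pak files at runtime, showing a W_PakPathLoader widget on BeginPlay.
; LoadPak mounts and registers the given file through PakManager, finds the first cooked BP_Main entry, and spawns that class at the actor's location.
; Only one pak asset stays loaded at a time; ClearPak destroys it and unmounts the pak, with debug prints reporting each step.
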(event Custom|LoadPak
  (params (FilePath :type String))
  (bind _returnvalue (Subsystems|GetPakManager))
  ;[0.0904 1 0.5528] MOUNT PAK
  (Development|PrintString (Utilities|String|Append "Pak File: " FilePath))
  (bind _output_get (Variables|Default|SetPak%20File%20Path FilePath))
  (Utilities|IsValid (Variables|Default|GetPakAsset)
    (:Is%20Valid
      (Development|PrintString "PAK ALREADY LOADED!! "))
    (:Is%20Not%20Valid
      (bind _bismountsuccessful (Class|PakManager|MountandRegisterPak _returnvalue _output_get))
      (Development|PrintString (Utilities|String|Append "Pak Mounted: " (Utilities|String|ToString(Boolean) _bismountsuccessful) " at "))
      (if _bismountsuccessful
        (bind _array_element (Utilities|Array|ForEachLoopwithBreak (Class|PakManager|GetPakContent _returnvalue (Variables|Default|GetPak%20File%20Path) true) :!label _label)
          (:LoopBody
            (if (Utilities|String|Contains _array_element "BP_Main")
              (bind _output_get_2 (Variables|Default|SetPreview%20Pak%20Path _array_element))
              (Development|PrintString (Utilities|String|Append "Pak Loading: " _output_get_2))
              (goto _label Break)))
          (:Completed
            (if (not (Utilities|Array|IsEmpty (Variables|Default|GetPreview%20Pak%20Path)))
              (bind _asactor (Utilities|Casting|CastToActorClass (Class|PakManager|LoadPakObjClassReference _returnvalue (Variables|Default|GetPreview%20Pak%20Path))))
              (bind _returnvalue_2 (Game|SpawnActorfromClass _asactor (Math|Transform|MakeTransform (Transformation|GetActorLocation) "0, 0, 0" "1.000000,1.000000,1.000000") "AlwaysSpawn" 0 0))
              (Variables|Default|SetPakAsset _returnvalue_2)
              (Development|PrintString "PAK Loaded!! "))))))))

(event Custom|ClearPak
  (bind _pakasset (Variables|Default|GetPakAsset))
  ;[1 0.3179 0] UNMOUNT PAK
  (Utilities|IsValid (Variables|Default|GetPakAsset)
    (:Is%20Valid
      (Development|PrintString (Utilities|String|Append "Clear Asset: " (Utilities|GetDisplayName _pakasset)))
      (Actor|DestroyActor _pakasset)
      (bind _returnvalue (Class|PakManager|UnmountPakFile (Subsystems|GetPakManager) (Variables|Default|GetPak%20File%20Path)))
      (Development|PrintString (Utilities|String|Append "Pak UnMounted: " (Utilities|String|ToString(Boolean) _returnvalue))))
    (:Is%20Not%20Valid
      (Development|PrintString "NOTHING TO CLEAR!! "))))

(event EventBeginPlay
  ;[1 1 0] STARTUP
  (bind _returnvalue (UserInterface|CreateWidget "/Game/Widgets/W_PakPathLoader.W_PakPathLoader_C"))
  (UserInterface|Viewport|AddtoViewport _returnvalue 0))

(fn ConstructionScript)